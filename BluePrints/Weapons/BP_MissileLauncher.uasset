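; BP_MissileLauncher is an actor that launches BP_Missile actors automatically at a regular interval.
; Tick accumulates delta time and spawns a missile each time the total exceeds SpawnInterval, then resets the timer.
; Each missile inherits the launcher's rotation, is scaled up, and gets a random world-space Y and Z offset from the launcher's location.
; Spawning adjusts for collisions and is skipped if no clear spot is found.
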(event `self.ReceiveBeginPlay`)

(event `self.ReceiveActorBeginOverlap`
  (params (OtherActor :type "Actor Object Reference")))

(event `self.ReceiveTick`
  (params (DeltaSeconds :type "Float (single-precision)"))
  (set `self.deltaSeconds` DeltaSeconds)
  (`|ExecutionSequence`
    (:`then_0`
      (`self.SpawnMissile`))))

(event `SpawnMissile`
  (bind _output_get (set `self.tmpInterval` (+ (`self.deltaSeconds`) (`self.tmpInterval`))))
  (if (> _output_get (`self.spawnInterval`))
    (set `self.tmpInterval` 0.0)
    (`|SpawnActorFromClass` "/Game/BluePrints/Weapons/BP_Missile.BP_Missile_C" (`KismetMathLibrary.MakeTransform` (`KismetMathLibrary.MakeVector` (.x (`self.K2_GetActorLocation`)) (+ (.y (`self.K2_GetActorLocation`)) (`KismetMathLibrary.RandomFloatInRange` -1500.0 1500.0)) (+ (.z (`self.K2_GetActorLocation`)) (`KismetMathLibrary.RandomFloatInRange` -350.0 350.0))) (`self.K2_GetActorRotation`) (2.0 2.0 2.0)) "AdjustIfPossibleButDontSpawnIfColliding" "OverrideRootScale")))

(fn `UserConstructionScript`)