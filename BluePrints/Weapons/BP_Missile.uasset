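; BP_Missile is a weapon projectile that explodes on impact and damages hover vehicles.
; It destroys itself after five seconds, or on a mesh hit that spawns a CarExplotion at the impact point and reduces a struck hover's health.
; Each tick stores delta time and spins the mesh by a fixed, frame-rate-dependent step.
; Throttle force and initial-velocity logic exist but are disconnected, so this graph applies no propulsion.
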(event `self.ReceiveBeginPlay`
  ;[1 1 1] Init
  (`KismetSystemLibrary.Delay` 5.0)
  (`self.K2_DestroyActor`))

(event `SetVariables`
  (params (deltaSeconds :type "Float (double-precision)"))
  ;[1 1 1] Set Variables
  (bind _output_get (set `self.deltaSeconds` deltaSeconds))
  (set `self.invertedDeltaSeconds` (- 1.0 _output_get)))

(event `Throttle`
  (bind _missilemesh (`self.MissileMesh`))
  ;[1 1 1] Force
  (`PrimitiveComponent.AddForce` _missilemesh (* (`SceneComponent.GetForwardVector` _missilemesh) (* (`self.MissileThrottle`) (`self.invertedDeltaSeconds`))) "None" true))

(event `self.ReceiveTick`
  (params (DeltaSeconds :type "Float (single-precision)"))
  ;[1 1 1] Tick
  (`|ExecutionSequence`
    (:`then_0`
      (`self.SetVariables` DeltaSeconds))
    (:`then_2`
      (`self.MissileRotation`))))

(event `self.MissileMesh.OnComponentHit`
  (params (OtherActor :type "Actor Object Reference") (OtherComp :type "PrimitiveComponent Object Reference") (NormalImpulse :type "Vector Structure") (Hit :type "HitResult Structure (by ref)"))
  ;[1 1 1] Hit
  (`self.MissileHit` false)
  (bind _ashover (cast `/Game/ThirdPersonBP/Blueprints/hover` OtherActor))
  (`/Game/ThirdPersonBP/Blueprints/hover.decreaseHealth` _ashover 10.0))

(event `MissileHit`
  (params (NewParam :type Boolean))
  ;[1 1 1] Destroy
  (`|SpawnActorFromClass` "/Game/ThirdPersonBP/Blueprints/CarExplotion.CarExplotion_C" (`KismetMathLibrary.MakeTransform` (`.ImpactPoint` (`GameplayStatics.BreakHitResult` (stale `self.MissileMesh.OnComponentHit` Hit)))) "Undefined" "OverrideRootScale")
  (`self.K2_DestroyActor`))

(event `MissileRotation`
  (`SceneComponent.K2_AddLocalRotation` (`self.MissileMesh`) (struct :`Roll` 10.0) false false))

(fn `UserConstructionScript`)