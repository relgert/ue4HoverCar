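; Homing missile that chases a Hover vehicle, spawning elevated behind its direction of travel and expiring after a fixed lifetime.
; Each tick drives physics velocity along the forward vector, spins the mesh and interpolates rotation toward the target, aiming higher when far away.
; Homing stops permanently once the aim error exceeds FollowAccuracy.
; On hit it spawns an explosion, destroys itself and damages any Hover struck.
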(event `setHomingTarget`
  ;[1 1 1] Set Target
  (bind _outactors (`GameplayStatics.GetAllActorsOfClass` "/Game/ThirdPersonBP/Blueprints/hover.hover_C"))
  (for _array_element _outactors
    (set `self.Target` (`/Game/ThirdPersonBP/Blueprints/hover.CarMesh` _array_element))))

(event `/Game/BluePrints/Weapons/BP_Missile.ReceiveBeginPlay`
  (bind _missilemesh (`self.MissileMesh`))
  ;[1 1 1] Init
  (`PrimitiveComponent.SetPhysicsLinearVelocity` _missilemesh (* (`SceneComponent.GetForwardVector` _missilemesh) (`self.InitialVelocity`)) false "None")
  (`self.setHomingTarget`)
  (`self.set Initial Location`)
  (`self.Set Initial Rotation`)
  (`KismetSystemLibrary.Delay` 15.0)
  (`self.K2_DestroyActor`))

(event `HomingRotation`
  (bind _target (`self.Target`))
  (bind _returnvalue (`SceneComponent.K2_GetComponentLocation` _target))
  (bind _returnvalue_2 (`SceneComponent.K2_GetComponentLocation` (`self.MissileMesh`)))
  (bind _returnvalue_3 (`SceneComponent.K2_GetComponentRotation` (`self.MissileMesh`)))
  (bind _returnvalue_4 (`KismetMathLibrary.FindLookAtRotation` _returnvalue_2 (`KismetMathLibrary.MakeVector` (.x _returnvalue) (.y _returnvalue) (+ (.z _returnvalue) (`self.targetHeight`)))))
  (if (and (`self.follow`) (`KismetSystemLibrary.IsValid` _target))
    (`SceneComponent.K2_SetWorldRotation` (`self.MissileMesh`) (`KismetMathLibrary.RInterpTo` _returnvalue_3 _returnvalue_4 (`self.deltaSeconds`) (`self.interpSpeed`)) true false)
    (if (> (`KismetMathLibrary.VSize` (- (`KismetMathLibrary.Conv_RotatorToVector` _returnvalue_4) (`KismetMathLibrary.Conv_RotatorToVector` _returnvalue_3))) (`self.FollowAccuracy`))
      (set `self.follow` false)
      (elif (> (`KismetMathLibrary.VSize` (- _returnvalue_2 _returnvalue)) 1500.0)
        (set `self.targetHeight` 300.0)
        (else
          (set `self.targetHeight` 50.0))))))

(event `SetVariables`
  (params (deltaSeconds :type "Float (double-precision)"))
  ;[1 1 1] Set Variables
  (bind _output_get (set `self.deltaSeconds` deltaSeconds))
  (set `self.invertedDeltaSeconds` (- 1.0 _output_get)))

(event `Throttle`
  (bind _missilemesh (`self.MissileMesh`))
  ;[1 1 1] Force
  (`PrimitiveComponent.SetPhysicsLinearVelocity` _missilemesh (* (`SceneComponent.GetForwardVector` _missilemesh) (* (`self.MissileThrottle`) (`self.invertedDeltaSeconds`))) false "None"))

(event `/Game/BluePrints/Weapons/BP_Missile.ReceiveTick`
  (params (DeltaSeconds :type "Float (single-precision)"))
  ;[1 1 1] Tick
  (`|ExecutionSequence`
    (:`then_0`
      (`self.SetVariables` DeltaSeconds))
    (:`then_1`
      (`self.Throttle`))
    (:`then_2`
      (`self.MissileRotation`))
    (:`then_3`
      (`self.HomingRotation`))))

(event `self.MissileMesh.OnComponentHit`
  (params (OtherActor :type "Actor Object Reference") (OtherComp :type "PrimitiveComponent Object Reference") (NormalImpulse :type "Vector Structure") (Hit :type "HitResult Structure (by ref)"))
  ;[1 1 1] Hit
  (`self.MissileHit` false)
  (bind _ashover (cast `/Game/ThirdPersonBP/Blueprints/hover` OtherActor))
  (`/Game/ThirdPersonBP/Blueprints/hover.decreaseHealth` _ashover 100.0))

(event `MissileHit`
  (params (NewParam :type Boolean))
  ;[1 1 1] Destroy
  (`|SpawnActorFromClass` "/Game/ThirdPersonBP/Blueprints/CarExplotion.CarExplotion_C" (`KismetMathLibrary.MakeTransform` (`.ImpactPoint` (`GameplayStatics.BreakHitResult` (stale `self.MissileMesh.OnComponentHit` Hit)))) "Undefined" "OverrideRootScale")
  (`self.K2_DestroyActor`))

(event `MissileRotation`
  ;[1 1 1] Missile Rotation
  (`SceneComponent.K2_AddLocalRotation` (`self.MissileMesh`) (struct :`Roll` 10.0) false false))

(event `set Initial Location`
  (bind _target (`self.Target`))
  ;[1 1 1] Set Iniitial Location
  (`SceneComponent.K2_SetWorldLocation` (`self.MissileMesh`) (`KismetMathLibrary.MakeVector` (.x (+ (`SceneComponent.K2_GetComponentLocation` _target) (* (`KismetMathLibrary.Normal` (`SceneComponent.GetComponentVelocity` _target)) -2000.0))) (.y (+ (`SceneComponent.K2_GetComponentLocation` _target) (* (`KismetMathLibrary.Normal` (`SceneComponent.GetComponentVelocity` _target)) -2000.0))) 1000.0) false false))

(event `Set Initial Rotation`
  (`SceneComponent.K2_SetWorldRotation` (`self.MissileMesh`) (`KismetMathLibrary.FindLookAtRotation` (`SceneComponent.K2_GetComponentLocation` (`self.MissileMesh`)) (`KismetMathLibrary.MakeVector` (.x (`SceneComponent.K2_GetComponentLocation` (`self.Target`))) 0.0 (.z (`SceneComponent.K2_GetComponentLocation` (`self.Target`))))) false false))

(fn `UserConstructionScript`)