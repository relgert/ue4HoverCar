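; BP_Laser is a rotating laser weapon that damages hover actors caught by its traces.
; Each tick it fires five randomly offset line traces along the emitter's negative up axis and uses the nearest hit to set beam length and spark position.
; The stored hit actor takes random damage every tick if it is a hover, and is never cleared when traces miss.
; The mesh then yaws at a constant, frame-rate-independent speed.
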(event `self.ReceiveBeginPlay`
  (bind _p_laser (`self.P_Laser`))
  (`ParticleSystemComponent.SetBeamSourcePoint` _p_laser 0 (`SceneComponent.K2_GetComponentLocation` _p_laser) 0))

(event `self.ReceiveTick`
  (params (DeltaSeconds :type "Float (single-precision)"))
  (`|ExecutionSequence`
    (:`then_0`
      (`self.UpdateLaser`))
    (:`then_1`
      (`self.RotateLaser`))))

(event `UpdateLaser`
  (bind _returnvalue (`KismetMathLibrary.RandomFloatInRange` -100.0 1000.0))
  (bind _p_laser (`self.P_Laser`))
  (bind _tracelenght (`self.TraceLenght`))
  (bind _p_laser_2 (`self.P_Laser`))
  (bind _returnvalue_2 (`SceneComponent.K2_GetComponentLocation` _p_laser))
  (bind _returnvalue_3 (+ (`SceneComponent.K2_GetComponentLocation` _p_laser_2) (* (`SceneComponent.GetUpVector` _p_laser_2) (* (`self.min length`) -1.0))))
  (set `self.min length` _tracelenght)
  (for _ (range 1 6)
    (bind (_outhit _returnvalue_4) (`KismetSystemLibrary.LineTraceSingle` _returnvalue_2 (`KismetMathLibrary.MakeVector` (+ (.x (+ _returnvalue_2 (* (`SceneComponent.GetUpVector` _p_laser) (* _tracelenght -1.0)))) _returnvalue) (+ (.y (+ _returnvalue_2 (* (`SceneComponent.GetUpVector` _p_laser) (* _tracelenght -1.0)))) _returnvalue) (.z (+ _returnvalue_2 (* (`SceneComponent.GetUpVector` _p_laser) (* _tracelenght -1.0))))) "TraceTypeQuery1"))
    (if _returnvalue_4
      (bind (_bblockinghit _binitialoverlap _time _location _impactpoint _normal _impactnormal _physmat _hitactor _hitcomponent _hitbonename _hititem _tracestart) (`GameplayStatics.BreakHitResult` _outhit))
      (bind _returnvalue_5 (`KismetMathLibrary.VSize` (- _tracestart _location)))
      (if (< _returnvalue_5 (`self.min length`))
        (set `self.min length` _returnvalue_5)
        (set `self.HitActor` _hitactor))))
  (`ParticleSystemComponent.SetBeamTargetPoint` _p_laser_2 0 _returnvalue_3 0)
  (`SceneComponent.K2_SetWorldLocation` (`self.P_Sparks`) _returnvalue_3 false false)
  (bind _ashover (cast `/Game/ThirdPersonBP/Blueprints/hover` (`self.HitActor`)))
  (`/Game/ThirdPersonBP/Blueprints/hover.decreaseHealth` _ashover (`KismetMathLibrary.RandomFloatInRange` 37.0 66.0)))

(event `RotateLaser`
  (`SceneComponent.K2_AddLocalRotation` (`self.StaticMeshComponent`) (`KismetMathLibrary.MakeRotator` 0.0 0.0 (* (`GameplayStatics.GetWorldDeltaSeconds`) 80.0)) true false))

(fn `UserConstructionScript`)